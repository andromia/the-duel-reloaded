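; Melee sword pickup that attaches to the first ThirdPersonCharacter to touch it and damages other characters when swung.
; Pickup snaps it to the "Sword" socket, sets wielder references and opens the hit gate.
; Slash resets a DoOnce, so capsule overlaps during an active animation trigger one damage pass over overlapping characters.
; The block check reads the wielder's BLOCK flag, briefly setting its EnemyBlocked instead of dealing damage.
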(event OnComponentBeginOverlap(Capsule)
  (params (OverlappedComponent :type Primitive%20Component%20Object%20Reference) (OtherActor :type Actor%20Object%20Reference) (OtherComp :type Primitive%20Component%20Object%20Reference) (OtherBodyIndex :type Integer) (bFromSweep :type Boolean) (SweepResult :type Hit%20Result%20Structure%20%28by%20ref%29))
  (bind _character (Variables|Default|GetCharacter))
  (bind _capsule (Variables|Default|GetCapsule))
  (bind _overlappingactors (Collision|GetOverlappingActors _capsule "/Game/ThirdPersonBP/Blueprints/ThirdPersonCharacter.ThirdPersonCharacter_C" :!class /Script/Engine.PrimitiveComponent))
  ;[1 1 1] hit detection, need to be reworked
  (Utilities|FlowControl|Gate true
    (:Exit
      (if (Variables|/Game/ThirdPersonBP/Blueprints/ThirdPersonCharacter.ThirdPersonCharacter_C|GetAnimActive (stale Collision|EventActorBeginOverlap _output_get))
        (if (!= OtherActor (stale Collision|EventActorBeginOverlap _output_get))
          (Utilities|FlowControl|DoOnce false
            (:Completed
              (Development|PrintString "Hello")
              (for (_array_element _array_index) _overlappingactors
                (if (not (== _array_element _character))
                  (if (Variables|/Game/ThirdPersonBP/Blueprints/ThirdPersonCharacter.ThirdPersonCharacter_C|GetBLOCK _character)
                    (Variables|/Game/ThirdPersonBP/Blueprints/ThirdPersonCharacter.ThirdPersonCharacter_C|SetEnemyBlocked? _character true)
                    (Utilities|FlowControl|Delay 0.2)
                    (Variables|/Game/ThirdPersonBP/Blueprints/ThirdPersonCharacter.ThirdPersonCharacter_C|SetEnemyBlocked? _character false)
                    (else
                      (Game|Damage|ApplyDamage (.AsThird%20Person%20Character (Utilities|Casting|CastToThirdPersonCharacter (Utilities|Array|Get(acopy) _overlappingactors _array_index))) 2e+01 (Game|GetInstigatorController _character) _character "/Script/Engine.DamageType"))))))))))))

(event Custom|Slash
  (bind _character (Variables|Default|GetCharacter))
  (bind _capsule (Variables|Default|GetCapsule))
  (bind _overlappingactors (Collision|GetOverlappingActors _capsule "/Game/ThirdPersonBP/Blueprints/ThirdPersonCharacter.ThirdPersonCharacter_C" :!class /Script/Engine.PrimitiveComponent))
  ;[1 1 1] hit detection, need to be reworked
  (Utilities|FlowControl|DoOnce false) ; enters at Reset
)

(event Collision|EventActorBeginOverlap
  (params (OtherActor :type Actor%20Object%20Reference))
  (bind _asthird_person_character (Utilities|Casting|CastToThirdPersonCharacter OtherActor))
  (bind _capsule (Variables|Default|GetCapsule))
  (bind _overlappingactors (Collision|GetOverlappingActors _capsule "/Game/ThirdPersonBP/Blueprints/ThirdPersonCharacter.ThirdPersonCharacter_C" :!class /Script/Engine.PrimitiveComponent))
  ;[1 1 1] bind sword to owner
  (if (== (Utilities|GetClass OtherActor) "/Game/ThirdPersonBP/Blueprints/ThirdPersonCharacter.ThirdPersonCharacter_C")
    (Utilities|FlowControl|DoOnce false
      (:Completed
        (Transformation|AttachComponentToComponent (Variables|/Script/Engine.Character|GetMesh _asthird_person_character) "Sword" "SnapToTarget" "SnapToTarget" "SnapToTarget" true)
        (Variables|/Game/ThirdPersonBP/Blueprints/ThirdPersonCharacter.ThirdPersonCharacter_C|SetHasSword _asthird_person_character true)
        (Variables|/Game/ThirdPersonBP/Blueprints/ThirdPersonCharacter.ThirdPersonCharacter_C|SetSwordReference _asthird_person_character self)
        (bind _output_get (Variables|Default|SetCharacter _asthird_person_character))
        ;[1 1 1] hit detection, need to be reworked
        (Utilities|FlowControl|Gate true) ; enters at Open
      ))))

(fn ConstructionScript)